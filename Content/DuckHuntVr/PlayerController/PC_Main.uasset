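; PC_Main is the VR player controller for Duck Hunt VR, routing motion controller input to the left and right hands.
; On BeginPlay it adds Enhanced Input mapping contexts for each hand's animations and actions.
; Touch, trigger and grip actions write pointing, thumb-up and axis values to the hand controllers, while shoot actions call ShootIfHasGun.
; Helper getters resolve each hand through the possessed BP_VrPawn, with validity checks before use.
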(event Input|EnhancedActionEvents|EnhancedInputActionIA_LeftControllerGrip
  (params (ActionValue :type Float%20%28double-precision%29) (ElapsedSeconds :type Float%20%28double-precision%29) (TriggeredSeconds :type Float%20%28double-precision%29) (InputAction :type Input%20Action%20Object%20Reference :default "/Game/DuckHuntVr/Characters/Player/Hands/Controller/Input/Actions/IA_LeftControllerGrip.IA_LeftControllerGrip"))
  ;[1 1 1] Left Hand Controller Animations
  (:Triggered
    (bind _lefthandcontroller (Utilities|GetLeftHandController :!label _label)
      (:Valid
        (Variables|/Script/DuckHuntVr.HandController|SetGripAxis _lefthandcontroller ActionValue))))
  (:Completed
    (goto _label)))

(event Input|EnhancedActionEvents|EnhancedInputActionIA_LeftControllerPointCapTouch
  (params (ActionValue :type Boolean) (ElapsedSeconds :type Float%20%28double-precision%29) (TriggeredSeconds :type Float%20%28double-precision%29) (InputAction :type Input%20Action%20Object%20Reference :default "/Game/DuckHuntVr/Characters/Player/Hands/Controller/Input/Actions/IA_LeftControllerPointCapTouch.IA_LeftControllerPointCapTouch"))
  ;[1 1 1] Left Hand Controller Animations
  (:Started
    (bind _lefthandcontroller (Utilities|GetLeftHandController :!label _label)
      (:Valid
        (Variables|/Script/DuckHuntVr.HandController|SetIsPointing _lefthandcontroller ActionValue))))
  (:Completed
    (goto _label)))

(event Input|EnhancedActionEvents|EnhancedInputActionIA_LeftControllerTrigger
  (params (ActionValue :type Float%20%28double-precision%29) (ElapsedSeconds :type Float%20%28double-precision%29) (TriggeredSeconds :type Float%20%28double-precision%29) (InputAction :type Input%20Action%20Object%20Reference :default "/Game/DuckHuntVr/Characters/Player/Hands/Controller/Input/Actions/IA_LeftControllerTrigger.IA_LeftControllerTrigger"))
  ;[1 1 1] Left Hand Controller Animations
  (:Triggered
    (bind _lefthandcontroller (Utilities|GetLeftHandController :!label _label)
      (:Valid
        (Variables|/Script/DuckHuntVr.HandController|SetTriggerAxis _lefthandcontroller ActionValue))))
  (:Completed
    (goto _label)))

(event Input|EnhancedActionEvents|EnhancedInputActionIA_LeftControllerThumbCapTouch
  (params (ActionValue :type Boolean) (ElapsedSeconds :type Float%20%28double-precision%29) (TriggeredSeconds :type Float%20%28double-precision%29) (InputAction :type Input%20Action%20Object%20Reference :default "/Game/DuckHuntVr/Characters/Player/Hands/Controller/Input/Actions/IA_LeftControllerThumbCapTouch.IA_LeftControllerThumbCapTouch"))
  ;[1 1 1] Left Hand Controller Animations
  (:Started
    (bind _lefthandcontroller (Utilities|GetLeftHandController :!label _label)
      (:Valid
        (Variables|/Script/DuckHuntVr.HandController|SetIsThumbUp _lefthandcontroller ActionValue))))
  (:Completed
    (goto _label)))

(event Input|EnhancedActionEvents|EnhancedInputActionIA_LeftControllerShoot
  (params (ActionValue :type Boolean) (ElapsedSeconds :type Float%20%28double-precision%29) (TriggeredSeconds :type Float%20%28double-precision%29) (InputAction :type Input%20Action%20Object%20Reference :default "/Game/DuckHuntVr/Characters/Player/Hands/Controller/Input/Actions/IA_LeftControllerShoot.IA_LeftControllerShoot"))
  ;[1 1 1] Left Hand Controller Actions
  (bind _lefthandcontroller (Utilities|GetLeftHandController)
    (:Valid
      (Class|HandController|ShootifHasGun _lefthandcontroller))))

(event Input|EnhancedActionEvents|EnhancedInputActionIA_RightControllerPointCapTouch
  (params (ActionValue :type Boolean) (ElapsedSeconds :type Float%20%28double-precision%29) (TriggeredSeconds :type Float%20%28double-precision%29) (InputAction :type Input%20Action%20Object%20Reference :default "/Game/DuckHuntVr/Characters/Player/Hands/Controller/Input/Actions/IA_RightControllerPointCapTouch.IA_RightControllerPointCapTouch"))
  ;[1 1 1] Right Hand Controller Animations
  (:Started
    (bind _righthandcontroller (Utilities|GetRightHandController :!label _label)
      (:Valid
        (Variables|/Script/DuckHuntVr.HandController|SetIsPointing _righthandcontroller ActionValue))))
  (:Completed
    (goto _label)))

(event Input|EnhancedActionEvents|EnhancedInputActionIA_RightControllerThumbCapTouch
  (params (ActionValue :type Boolean) (ElapsedSeconds :type Float%20%28double-precision%29) (TriggeredSeconds :type Float%20%28double-precision%29) (InputAction :type Input%20Action%20Object%20Reference :default "/Game/DuckHuntVr/Characters/Player/Hands/Controller/Input/Actions/IA_RightControllerThumbCapTouch.IA_RightControllerThumbCapTouch"))
  ;[1 1 1] Right Hand Controller Animations
  (:Started
    (bind _righthandcontroller (Utilities|GetRightHandController :!label _label)
      (:Valid
        (Variables|/Script/DuckHuntVr.HandController|SetIsThumbUp _righthandcontroller ActionValue))))
  (:Completed
    (goto _label)))

(event Input|EnhancedActionEvents|EnhancedInputActionIA_RightControllerTrigger
  (params (ActionValue :type Float%20%28double-precision%29) (ElapsedSeconds :type Float%20%28double-precision%29) (TriggeredSeconds :type Float%20%28double-precision%29) (InputAction :type Input%20Action%20Object%20Reference :default "/Game/DuckHuntVr/Characters/Player/Hands/Controller/Input/Actions/IA_RightControllerTrigger.IA_RightControllerTrigger"))
  ;[1 1 1] Right Hand Controller Animations
  (:Triggered
    (bind _righthandcontroller (Utilities|GetRightHandController :!label _label)
      (:Valid
        (Variables|/Script/DuckHuntVr.HandController|SetTriggerAxis _righthandcontroller ActionValue))))
  (:Completed
    (goto _label)))

(event Input|EnhancedActionEvents|EnhancedInputActionIA_RightControllerGrip
  (params (ActionValue :type Float%20%28double-precision%29) (ElapsedSeconds :type Float%20%28double-precision%29) (TriggeredSeconds :type Float%20%28double-precision%29) (InputAction :type Input%20Action%20Object%20Reference :default "/Game/DuckHuntVr/Characters/Player/Hands/Controller/Input/Actions/IA_RightControllerGrip.IA_RightControllerGrip"))
  ;[1 1 1] Right Hand Controller Animations
  (:Triggered
    (bind _righthandcontroller (Utilities|GetRightHandController :!label _label)
      (:Valid
        (Variables|/Script/DuckHuntVr.HandController|SetGripAxis _righthandcontroller ActionValue))))
  (:Completed
    (goto _label)))

(event Input|EnhancedActionEvents|EnhancedInputActionIA_RightControllerShoot
  (params (ActionValue :type Boolean) (ElapsedSeconds :type Float%20%28double-precision%29) (TriggeredSeconds :type Float%20%28double-precision%29) (InputAction :type Input%20Action%20Object%20Reference :default "/Game/DuckHuntVr/Characters/Player/Hands/Controller/Input/Actions/IA_RightControllerShoot.IA_RightControllerShoot"))
  ;[1 1 1] Right Hand Controller Actions
  (bind _righthandcontroller (Utilities|GetRightHandController)
    (:Valid
      (Class|HandController|ShootifHasGun _righthandcontroller))))

(event EventBeginPlay
  (bind _returnvalue (PlayerController|LocalPlayerSubsystems|GetEnhancedInputLocalPlayerSubsystem))
  (Input|AddMappingContext _returnvalue "/Game/DuckHuntVr/Characters/Player/Hands/Controller/Input/IMC_LeftControllerHandAnim.IMC_LeftControllerHandAnim" 0 "(bIgnoreAllPressedKeysUntilRelease=True,bForceImmediately=False,bNotifyUserSettings=False)")
  (Input|AddMappingContext _returnvalue "/Game/DuckHuntVr/Characters/Player/Hands/Controller/Input/IMC_LeftControllerHandActions.IMC_LeftControllerHandActions" 0 "(bIgnoreAllPressedKeysUntilRelease=True,bForceImmediately=False,bNotifyUserSettings=False)")
  (Input|AddMappingContext _returnvalue "/Game/DuckHuntVr/Characters/Player/Hands/Controller/Input/IMC_RightControllerHandAnim.IMC_RightControllerHandAnim" 0 "(bIgnoreAllPressedKeysUntilRelease=True,bForceImmediately=False,bNotifyUserSettings=False)")
  (Input|AddMappingContext _returnvalue "/Game/DuckHuntVr/Characters/Player/Hands/Controller/Input/IMC_RightControllerHandActions.IMC_RightControllerHandActions" 0 "(bIgnoreAllPressedKeysUntilRelease=True,bForceImmediately=False,bNotifyUserSettings=False)"))

(fn ConstructionScript)