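; Right-hand component for the VR player that tracks controller input for hand pose and fires a held gun.
; On BeginPlay it adds the right-hand animation and action Enhanced Input mapping contexts to the local player.
; Capacitive touch, trigger and grip inputs update pointing, thumb-up and axis variables.
; The shoot action calls Shoot with the right side on the gun, found by casting the component's first child.
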(event Input|EnhancedActionEvents|EnhancedInputActionIA_RightControllerPointCapTouch
  (params (ActionValue :type Boolean) (ElapsedSeconds :type Float%20%28double-precision%29) (TriggeredSeconds :type Float%20%28double-precision%29) (InputAction :type Input%20Action%20Object%20Reference :default "/Game/DuckHuntVr/Characters/Player/Hands/Right/Input/Actions/IA_RightControllerPointCapTouch.IA_RightControllerPointCapTouch"))
  (:Started
    (Variables|Default|SetIsPointing ActionValue :!label _label))
  (:Completed
    (goto _label)))

(event Input|EnhancedActionEvents|EnhancedInputActionIA_RightControllerThumbCapTouch
  (params (ActionValue :type Boolean) (ElapsedSeconds :type Float%20%28double-precision%29) (TriggeredSeconds :type Float%20%28double-precision%29) (InputAction :type Input%20Action%20Object%20Reference :default "/Game/DuckHuntVr/Characters/Player/Hands/Right/Input/Actions/IA_RightControllerThumbCapTouch.IA_RightControllerThumbCapTouch"))
  (:Started
    (Variables|Default|SetIsThumbUp ActionValue :!label _label))
  (:Completed
    (goto _label)))

(event Input|EnhancedActionEvents|EnhancedInputActionIA_RightControllerGrip
  (params (ActionValue :type Float%20%28double-precision%29) (ElapsedSeconds :type Float%20%28double-precision%29) (TriggeredSeconds :type Float%20%28double-precision%29) (InputAction :type Input%20Action%20Object%20Reference :default "/Game/DuckHuntVr/Characters/Player/Hands/Right/Input/Actions/IA_RightControllerGrip.IA_RightControllerGrip"))
  (:Triggered
    (Variables|Default|SetGripAxis ActionValue :!label _label))
  (:Completed
    (goto _label)))

(event Input|EnhancedActionEvents|EnhancedInputActionIA_RightControllerTrigger
  (params (ActionValue :type Float%20%28double-precision%29) (ElapsedSeconds :type Float%20%28double-precision%29) (TriggeredSeconds :type Float%20%28double-precision%29) (InputAction :type Input%20Action%20Object%20Reference :default "/Game/DuckHuntVr/Characters/Player/Hands/Right/Input/Actions/IA_RightControllerTrigger.IA_RightControllerTrigger"))
  (:Triggered
    (Variables|Default|SetTriggerAxis ActionValue :!label _label))
  (:Completed
    (goto _label)))

(event Input|EnhancedActionEvents|EnhancedInputActionIA_RightControllerShoot
  (params (ActionValue :type Boolean) (ElapsedSeconds :type Float%20%28double-precision%29) (TriggeredSeconds :type Float%20%28double-precision%29) (InputAction :type Input%20Action%20Object%20Reference :default "/Game/DuckHuntVr/Characters/Player/Hands/Right/Input/Actions/IA_RightControllerShoot.IA_RightControllerShoot"))
  (bind (_gunvalid _gun) (CallFunction|HasGun))
  (if _gunvalid
    (Class|Gun|Shoot _gun "Right")))

(event EventBeginPlay
  (bind _returnvalue (Game|GetPlayerController 0))
  (bind _returnvalue_2 (PlayerController|LocalPlayerSubsystems|GetEnhancedInputLocalPlayerSubsystem _returnvalue))
  (Input|AddMappingContext _returnvalue_2 "/Game/DuckHuntVr/Characters/Player/Hands/Right/Input/IMC_RightControllerHandAnim.IMC_RightControllerHandAnim" 0 "(bIgnoreAllPressedKeysUntilRelease=True,bForceImmediately=False,bNotifyUserSettings=False)")
  (Input|AddMappingContext _returnvalue_2 "/Game/DuckHuntVr/Characters/Player/Hands/Right/Input/IMC_RightControllerHandActions.IMC_RightControllerHandActions" 0 "(bIgnoreAllPressedKeysUntilRelease=True,bForceImmediately=False,bNotifyUserSettings=False)"))

(fn HasGun
  (bind _asgun (Utilities|Casting|CastToGun (Components|GetChildComponent 0))
    (:then
      (return true _asgun))
    (:CastFailed
      (return false 0))))