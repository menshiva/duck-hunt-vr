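; Left VR hand component for the Duck Hunt player that tracks controller input state, apparently for hand animation.
; On BeginPlay it adds the left-controller hand animation mapping context to the first player controller.
; Enhanced Input events store trigger and grip axes plus capacitive-touch pointing and thumb-up states in variables.
; HasGun casts the first child component to BP_Gun, returning whether it is valid and the gun itself.
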(event Input|EnhancedActionEvents|EnhancedInputActionIA_LeftControllerGrip
  (params (ActionValue :type Float%20%28double-precision%29) (ElapsedSeconds :type Float%20%28double-precision%29) (TriggeredSeconds :type Float%20%28double-precision%29) (InputAction :type Input%20Action%20Object%20Reference :default "/Game/DuckHuntVr/Characters/Player/Hands/Left/Input/Actions/IA_LeftControllerGrip.IA_LeftControllerGrip"))
  (:Triggered
    (Variables|Default|SetGripAxis ActionValue :!label _label))
  (:Completed
    (goto _label)))

(event Input|EnhancedActionEvents|EnhancedInputActionIA_LeftControllerPointCapTouch
  (params (ActionValue :type Boolean) (ElapsedSeconds :type Float%20%28double-precision%29) (TriggeredSeconds :type Float%20%28double-precision%29) (InputAction :type Input%20Action%20Object%20Reference :default "/Game/DuckHuntVr/Characters/Player/Hands/Left/Input/Actions/IA_LeftControllerPointCapTouch.IA_LeftControllerPointCapTouch"))
  (:Started
    (Variables|Default|SetIsPointing ActionValue :!label _label))
  (:Completed
    (goto _label)))

(event Input|EnhancedActionEvents|EnhancedInputActionIA_LeftControllerTrigger
  (params (ActionValue :type Float%20%28double-precision%29) (ElapsedSeconds :type Float%20%28double-precision%29) (TriggeredSeconds :type Float%20%28double-precision%29) (InputAction :type Input%20Action%20Object%20Reference :default "/Game/DuckHuntVr/Characters/Player/Hands/Left/Input/Actions/IA_LeftControllerTrigger.IA_LeftControllerTrigger"))
  (:Triggered
    (Variables|Default|SetTriggerAxis ActionValue :!label _label))
  (:Completed
    (goto _label)))

(event Input|EnhancedActionEvents|EnhancedInputActionIA_LeftControllerThumbCapTouch
  (params (ActionValue :type Boolean) (ElapsedSeconds :type Float%20%28double-precision%29) (TriggeredSeconds :type Float%20%28double-precision%29) (InputAction :type Input%20Action%20Object%20Reference :default "/Game/DuckHuntVr/Characters/Player/Hands/Left/Input/Actions/IA_LeftControllerThumbCapTouch.IA_LeftControllerThumbCapTouch"))
  (:Started
    (Variables|Default|SetIsThumbUp ActionValue :!label _label))
  (:Completed
    (goto _label)))

(event EventBeginPlay
  (Input|AddMappingContext (PlayerController|LocalPlayerSubsystems|GetEnhancedInputLocalPlayerSubsystem (Game|GetPlayerController 0)) "/Game/DuckHuntVr/Characters/Player/Hands/Left/Input/IMC_LeftControllerHandAnim.IMC_LeftControllerHandAnim" 0 "(bIgnoreAllPressedKeysUntilRelease=True,bForceImmediately=False,bNotifyUserSettings=False)"))

(fn HasGun
  (bind _asbp_gun (Utilities|Casting|CastToBP_Gun (Components|GetChildComponent 0))
    (:then
      (return true _asbp_gun))
    (:CastFailed
      (return false 0))))